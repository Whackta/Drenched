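; GargoyleProjectile is an enemy projectile actor that explodes when it overlaps the player's pawn.
; On that overlap it spawns an explosion particle effect at its location and destroys itself after a brief delay.
; Each tick it tumbles on all three local axes at one shared rate, YawPerSecond.
; The graph itself applies no damage and does no movement other than this rotation.
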(event `self.ReceiveActorBeginOverlap`
  (params (OtherActor :type "Actor Object Reference"))
  (if (== (`GameplayStatics.GetPlayerPawn` 0) OtherActor)
    (`GameplayStatics.SpawnEmitterAtLocation` "/Game/StarterContent/Particles/P_Explosion.P_Explosion" (`self.K2_GetActorLocation`))
    (`KismetSystemLibrary.Delay` 0.05)
    (`self.K2_DestroyActor`)))

(event `self.ReceiveTick`
  (params (DeltaSeconds :type "Float (single-precision)"))
  (bind _returnvalue (* DeltaSeconds (`self.YawPerSecond`)))
  (`self.K2_AddActorLocalRotation` (`KismetMathLibrary.MakeRotator` _returnvalue _returnvalue _returnvalue)))

(fn `UserConstructionScript`)