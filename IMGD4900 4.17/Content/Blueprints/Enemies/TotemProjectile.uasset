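; TotemProjectile is an enemy projectile that drops onto the player from above and leaves a BloodPool where it hits.
; On BeginPlay it activates its movement, waits TimeToGoUp, then jumps to the player's X/Y with slight random jitter, keeping its height.
; It then raises gravity scale sharply to fall.
; On hit it spawns the pool at its own transform before calling the parent hit logic.
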(event `self.ReceiveHit`
  (params (MyComp :type "PrimitiveComponent Object Reference") (Other :type "Actor Object Reference") (OtherComp :type "PrimitiveComponent Object Reference") (bSelfMoved :type Boolean) (HitLocation :type "Vector Structure") (HitNormal :type "Vector Structure") (NormalImpulse :type "Vector Structure") (Hit :type "HitResult Structure (by ref)"))
  (`|SpawnActorFromClass` "/Game/Blueprints/Blood/BloodPool.BloodPool_C" (`self.GetTransform`) "Undefined" "OverrideRootScale" null null)
  (`parent.ReceiveHit` null Other null false HitLocation HitNormal NormalImpulse Hit))

(event `self.ReceiveBeginPlay`
  (bind (_returnvalue_x _returnvalue_y _returnvalue_z) (`KismetMathLibrary.BreakVector` (`self.K2_GetActorLocation`)))
  (bind (_returnvalue_x_2 _returnvalue_y_2) (`KismetMathLibrary.BreakVector` (`self.K2_GetActorLocation` (`GameplayStatics.GetPlayerPawn` 0))))
  (`ActorComponent.Activate` (`self.ProjectileMovement`) false)
  (`KismetSystemLibrary.Delay` (`self.TimeToGoUp`))
  (`self.K2_SetActorLocation` (`KismetMathLibrary.MakeVector` (+ _returnvalue_x_2 (`KismetMathLibrary.RandomFloatInRange` -25.0 25.0)) (+ _returnvalue_y_2 (`KismetMathLibrary.RandomFloatInRange` -25.0 25.0)) _returnvalue_z))
  (set `ProjectileMovementComponent.ProjectileGravityScale` 15.0 (`self.ProjectileMovement`)))

(fn `UserConstructionScript`)