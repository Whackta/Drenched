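; TotemCharacter is an enemy totem that repeatedly fires barrages of projectiles and plays a sound when it spawns.
; After a random delay it plays the Barrage timeline at double rate, then schedules the next barrage when that finishes.
; A timeline event track spawns TotemProjectile actors at ProjectileSource with slight random roll and pitch and fixed yaw.
; ExtraDeathEffects stops the timeline on death.
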(event `self.ReceiveBeginPlay`
  (`parent.ReceiveBeginPlay`)
  (`GameplayStatics.PlaySound2D` null)
  (`KismetSystemLibrary.PrintString` "PLAY THE TOTEM SOUND!")
  (`self.StartBarrage`)
  (`TimelineComponent.SetPlayRate` (`self.Barrage`) 2.0))

(event `StartBarrage`
  (bind _returnvalue (`KismetMathLibrary.RandomFloatInRange` -2.0 2.0))
  (bind (_returnvalue_x _returnvalue_y _returnvalue_z) (`KismetMathLibrary.BreakVector` (`SceneComponent.K2_GetComponentLocation` (`self.ProjectileSource`))))
  (`KismetSystemLibrary.Delay` (`KismetMathLibrary.RandomFloatInRange` 2.0 4.0))
  (`KismetSystemLibrary.PrintString` "Start Barrage!")
  (`Timeline|Barrage` :!via `PlayFromStart` :!label _label
    (:`Finished`
      (`self.StartBarrage`))
    (:`NewTrack_2`
      (`|SpawnActorFromClass` "/Game/Blueprints/Enemies/TotemProjectile.TotemProjectile_C" (`KismetMathLibrary.MakeTransform` (`KismetMathLibrary.MakeVector` _returnvalue_x _returnvalue_y _returnvalue_z) (`KismetMathLibrary.MakeRotator` _returnvalue _returnvalue 90.0)) "Undefined" "OverrideRootScale" null null))))

(event `self.Extra Death Effects`
  (`KismetSystemLibrary.PrintString` "Stop barrage!")
  (goto _label :!via `Stop`))

(fn `UserConstructionScript`
  (`parent.UserConstructionScript`))