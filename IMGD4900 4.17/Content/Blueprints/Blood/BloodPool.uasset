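; Blood pool actor that spreads when the player dodges into it and can be detonated in a chain reaction.
; A dodge spawns a child pool ahead unless pools would overlap; the fast-fall check is a stub.
; BloodStrike waits briefly, triggers particles, recursively strikes child pools, spawns a BloodExplosion, then fades its decals and destroys itself.
; Spawn and particle collisions place randomly indexed blood decals, tracked for cleanup.
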(event `BloodStrike`
  ;[1 1 1] Blood Strike, delay 0.1 seconds before exploding
  (`KismetSystemLibrary.Delay` 0.1)
  (`self.explodeNode`)
  (`|SpawnActorFromClass` "/Game/Blueprints/Blood/BloodExplosion.BloodExplosion_C" (`SceneComponent.K2_GetComponentToWorld` (`self.Cylinder`)) "Undefined" "OverrideRootScale" null null)
  ;[1 1 1] Delete all Decals that this node has spawned
  (bind _result (`BlueprintSetLibrary.Set_ToArray` (`self.Decals`)))
  (for _array_element _result
    (`DecalComponent.SetFadeOut` _array_element 0.0 0.2 true))
  ;[1 1 1] Delete this Blood Pool Actor
  (`self.K2_DestroyActor`))

(event `self.ReceiveBeginPlay`
  ;[1 1 1] Init Edge Detector
  ;[1 1 1] Initialize Decal index to a random number
  (bind _returnvalue (`KismetMaterialLibrary.CreateDynamicMaterialInstance` "/Game/Materials/decal_blood.decal_blood"))
  (`MaterialInstanceDynamic.SetScalarParameterValue` _returnvalue "index" (`KismetMathLibrary.Conv_IntToDouble` (`KismetMathLibrary.FFloor` (* 8 (`KismetMathLibrary.RandomFloat`)))))
  (bind _returnvalue_2 (`GameplayStatics.SpawnDecalAtLocation` _returnvalue (128.0 128.0 128.0) (`SceneComponent.K2_GetComponentLocation` (`self.Cylinder`))))
  ;[1 1 1] Add Decal to array of add Decals
  (`BlueprintSetLibrary.Set_Add` (`self.Decals`) _returnvalue_2))

(event `self.Cylinder.OnComponentBeginOverlap`
  (params (OverlappedComponent :type "PrimitiveComponent Object Reference") (OtherActor :type "Actor Object Reference") (OtherComp :type "PrimitiveComponent Object Reference") (OtherBodyIndex :type Integer) (bFromSweep :type Boolean) (SweepResult :type "HitResult Structure (by ref)"))
  ;[1 1 1] Rising Edge Detector, when player enters
  (if (`self.canAdd`)
    (set `self.canAdd` false)
    ;[1 1 1] Check If Player is Dodging
    (bind _asplayer_character (cast `/Game/ThirdPersonBP/Blueprints/PlayerCharacter` (`GameplayStatics.GetPlayerPawn` 0)))
    (if (`/Game/ThirdPersonBP/Blueprints/PlayerCharacter.isDodging` _asplayer_character)
      ;[1 1 1] Check If current Blood Pool is Overlapping another Blood Pool
      (bind _isoverlapping (`self.isOverlappingClass` "BloodPool_C"))
      (if (not _isoverlapping)
        ;[1 1 1] Generate New Blood pool in the direction the player is moving
        (bind _returnvalue (`|SpawnActorFromClass` "BloodPool_C" (`KismetMathLibrary.MakeTransform` (+ (`self.K2_GetActorLocation`) (* (`SceneComponent.GetForwardVector` (`Actor.RootComponent` OtherActor)) (128.0 128.0 0.0))) (`self.K2_GetActorRotation`)) "DontSpawnIfColliding" "OverrideRootScale" null null))
        ;[1 1 1] After Spawn Check if this actor is intersecting any additonal blood pools, if so Delete self
        (bind _isoverlapping_2 (`self.isOverlappingClass` _returnvalue "BloodPool_C"))
        (if _isoverlapping_2
          (`self.K2_DestroyActor` _returnvalue)
          (else
            ;[1 1 1] Add new Blood pool to array of child pools
            (`BlueprintSetLibrary.Set_Add` (`self.Child`) _returnvalue))))
      (else
        ;[1 1 1] Check If Player is Fast Falling
        (bind _asplayer_character_2 (cast `/Game/ThirdPersonBP/Blueprints/PlayerCharacter` (`GameplayStatics.GetPlayerPawn` 0)))
        (if (`/Game/ThirdPersonBP/Blueprints/PlayerCharacter.isFastFalling` _asplayer_character_2)
          _)))))

(event `self.ReceiveActorEndOverlap`
  (params (OtherActor :type "Actor Object Reference"))
  ;[1 1 1] Reset Edge Detector
  (set `self.canAdd` true))

(event `self.ParticleSystem.OnParticleCollide`
  (params (EventName :type Name) (EmitterTime :type "Float (single-precision)") (ParticleTime :type Integer) (Location :type "Vector Structure") (Velocity :type "Vector Structure") (Direction :type "Vector Structure") (Normal :type "Vector Structure") (BoneName :type Name) (PhysMat :type "PhysicalMaterial Object Reference"))
  ;[1 1 1] Spawn Decal on particle hitting the floor
  (bind _returnvalue (`KismetMaterialLibrary.CreateDynamicMaterialInstance` "/Game/Materials/decal_blood.decal_blood"))
  (`MaterialInstanceDynamic.SetScalarParameterValue` _returnvalue "index" (`KismetMathLibrary.Conv_IntToDouble` (`KismetMathLibrary.FFloor` (* 8 (`KismetMathLibrary.RandomFloat`)))))
  (bind _returnvalue_2 (`GameplayStatics.SpawnDecalAtLocation` _returnvalue (128.0 128.0 128.0) Location))
  ;[1 1 1] Add Decal to array of add Decals
  (`BlueprintSetLibrary.Set_Add` (`self.Decals`) _returnvalue_2))

(fn `explodeNode`
  (`ActorComponent.Activate` (`self.ParticleSystem`) true)
  (bind _result (`BlueprintSetLibrary.Set_ToArray` (`self.Child`)))
  (for _array_element _result
    (bind _asblood_pool (cast `/Game/Blueprints/Blood/BloodPool` _array_element))
    (`self.BloodStrike` _asblood_pool)))

(fn `isOverlappingClass`
  (params (ClassType :type "Actor Class Reference"))
  (returns (isOverlapping :type Boolean) (OverlappingActors :type "Array of Actor Object Reference"))
  (bind _overlappingactors (`self.GetOverlappingActors` ClassType))
  (return (>= (`KismetArrayLibrary.Array_Length` _overlappingactors) 1) _overlappingactors))

(fn `UserConstructionScript`)