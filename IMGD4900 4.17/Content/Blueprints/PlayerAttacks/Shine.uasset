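; Shine is a short-lived player attack actor that knocks back and damages gargoyle enemies it overlaps, then destroys itself shortly after spawning.
; On overlap, it applies a velocity-change impulse with configurable horizontal and vertical strength, then updates Health through the gargoyle's EnemyHealth TakeDamage.
; The look-at rotation uses the gargoyle's location as both start and target, so knockback direction ignores the attack's position.
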(event `self.ReceiveBeginPlay`
  (`KismetSystemLibrary.Delay` 0.3)
  (`self.K2_DestroyActor`))

(event `self.ReceiveActorBeginOverlap`
  (params (OtherActor :type "Actor Object Reference"))
  (bind _asgargoyle_character (cast `/Game/Blueprints/Enemies/GargoyleCharacter` OtherActor))
  (bind (_returnvalue_x _returnvalue_y) (`KismetMathLibrary.BreakVector` (* (`KismetMathLibrary.GetForwardVector` (`KismetMathLibrary.FindLookAtRotation` (`self.K2_GetActorLocation` _asgargoyle_character) (`self.K2_GetActorLocation` OtherActor))) (`self.KnockbackIntensity`))))
  (`CharacterMovementComponent.AddImpulse` (`Character.CharacterMovement` _asgargoyle_character) (`KismetMathLibrary.MakeVector` _returnvalue_x _returnvalue_y (`self.KnockbackZ`)) true)
  (`/Engine/EditorBlueprintResources/StandardMacros.IsValid` _asgargoyle_character
    (:`Is Valid`
      (bind _newhealth (`/Game/Blueprints/Enemies/EnemyHealth.TakeDamage` (`/Game/Blueprints/Enemies/GargoyleCharacter.EnemyHealth` _asgargoyle_character) _asgargoyle_character (`/Game/Blueprints/Enemies/GargoyleCharacter.Health` _asgargoyle_character) (`self.Damage`)))
      (set `/Game/Blueprints/Enemies/GargoyleCharacter.Health` _newhealth _asgargoyle_character))))

(fn `UserConstructionScript`)