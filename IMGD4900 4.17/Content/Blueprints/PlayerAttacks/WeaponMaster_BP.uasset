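; WeaponMaster_BP is a base weapon Blueprint for player attacks that defines a common firing entry point.
; StartFire prints a debug message and calls Fire, a placeholder that only reports missing fire logic, apparently meant for child weapons to override.
; CameraAim reads the owning pawn's base aim rotation and forward vector, but does not yet use them to compute its target location.
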(event `StartFire`
  (`KismetSystemLibrary.PrintString` "TRY TO FIRE!")
  (`self.Fire`))

(fn `Camera Aim`
  (params (TargetLoc :type "Vector Structure"))
  (bind _returnvalue (`Pawn.GetBaseAimRotation` (`self.OwningPawn`)))
  (set `self.AimRotation` _returnvalue)
  (set `self.AimVetor` (`KismetMathLibrary.GetForwardVector` _returnvalue))
  (set `self.TargetLoc` TargetLoc))

(fn `Fire`
  (`KismetSystemLibrary.PrintString` "NO FIRE IMPLEMENTED D:"))

(fn `UserConstructionScript`)