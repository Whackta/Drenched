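; Player shotgun weapon that fires a horizontal fan of ShotgunProjectile_BP pellets from the muzzle along the aim direction.
; Fire loops to spawn the pellets, stepping ArcRotator's yaw offset evenly for each, then resets it for the next shot.
; Each pellet takes its damage from the player character's AttackPower.
; CanFire blocks further shots until ReloadDelay elapses; the random position jitter has a zero range, so has no effect.
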(event `self.Fire`
  (if (`self.CanFire`)
    (set `self.CanFire` false)
    (for _ (range 11)
      (`|SpawnActorFromClass` "/Game/Blueprints/PlayerAttacks/ShotgunProjectile_BP.ShotgunProjectile_BP_C" (`KismetMathLibrary.MakeTransform` (+ (+ (`SceneComponent.K2_GetComponentLocation` (`self.MuzzleLoc`)) (`self.AimVetor`)) (`KismetMathLibrary.RandomFloatInRange` 0.0)) (`KismetMathLibrary.MakeRotator` 0.0 (.pitch (`self.AimRotation`)) (+ (.yaw (`self.AimRotation`)) (`self.ArcRotator`)))) "Undefined" "OverrideRootScale" null (`/Game/ThirdPersonBP/Blueprints/PlayerCharacter.AttackPower` (cast `/Game/ThirdPersonBP/Blueprints/PlayerCharacter` (`GameplayStatics.GetPlayerPawn` 0) :!pure true)) null)
      (set `self.ArcRotator` (+ (`self.ArcRotator`) 2.0)))
    (set `self.ArcRotator` -10.0)
    (`KismetSystemLibrary.Delay` (`self.ReloadDelay`))
    (set `self.CanFire` true)))

(fn `UserConstructionScript`
  (`parent.UserConstructionScript`))