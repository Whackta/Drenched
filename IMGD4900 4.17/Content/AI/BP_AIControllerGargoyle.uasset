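; AI controller for the Gargoyle enemy that runs its behavior tree and targets the player character from BeginPlay.
; Perception updates for that target set CanSeePlayer from the first stimulus and feed LastSeenLocation from the target's position, falling back to the second stimulus's location.
; LookTowardsHit overwrites LastSeenLocation with the supplied hit vector.
; Debug spheres mark each recorded location, and target changes print on screen.
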(event `UpdateEnemyTarget`
  (params (TargetActor :type "Actor Object Reference"))
  (bind _output_get (set `self.Enemy` TargetActor))
  (`BlackboardComponent.SetValueAsObject` (`AIBlueprintHelperLibrary.GetBlackboard` null) "Enemy" _output_get)
  (`KismetSystemLibrary.PrintString` (`KismetStringLibrary.Concat_StrStr` "New target: " (`KismetSystemLibrary.GetDisplayName` _output_get))))

(event `self.OnPossess`
  (params (PossessedPawn :type "Pawn Object Reference"))
  (`self.UseBlackboard` "/Game/AI/BB_AIGargoyle.BB_AIGargoyle")
  (`self.RunBehaviorTree` "/Game/AI/BT_AIGargoyle.BT_AIGargoyle"))

(event `self.ReceiveBeginPlay`
  (`self.UpdateEnemyTarget` (`GameplayStatics.GetPlayerCharacter` 0)))

(event `self.AIPerception.OnPerceptionUpdated`
  (params (UpdatedActors :type "Array of Actor Object Reference"))
  (bind _returnvalue (`AIBlueprintHelperLibrary.GetBlackboard` null))
  (bind _returnvalue_2 (`self.K2_GetActorLocation` (`self.Enemy`)))
  (for _array_element UpdatedActors
    (if (== _array_element (`self.Enemy`))
      (bind _info (`AIPerceptionComponent.GetActorsPerception` (`self.AIPerception`) _array_element))
      (bind (_target _lastsensedstimuli) (break `ActorPerceptionBlueprintInfo` _info))
      (bind (_age _expirationage _strength _stimuluslocation _receiverlocation _tag _bsuccessfullysensed) (break `AIStimulus` (`|GetArrayItem` _lastsensedstimuli)))
      (`BlackboardComponent.SetValueAsBool` _returnvalue "CanSeePlayer" _bsuccessfullysensed)
      (if _bsuccessfullysensed
        (`BlackboardComponent.SetValueAsVector` _returnvalue "LastSeenLocation" _returnvalue_2)
        (`KismetSystemLibrary.DrawDebugSphere` _returnvalue_2 100.0 12 (struct :`R` 1.0 :`G` 1.0 :`B` 1.0 :`A` 1.0) 5.0 1.0)
        (else
          (bind (_age_2 _expirationage_2 _strength_2 _stimuluslocation_2 _receiverlocation_2 _tag_2 _bsuccessfullysensed_2) (break `AIStimulus` (`|GetArrayItem` _lastsensedstimuli 1)))
          (if _bsuccessfullysensed_2
            (`BlackboardComponent.SetValueAsVector` _returnvalue "LastSeenLocation" _stimuluslocation_2)
            (`KismetSystemLibrary.DrawDebugSphere` _stimuluslocation_2 100.0 12 (struct :`R` 1.0 :`G` 0.763839 :`A` 1.0) 5.0 1.0)))))))

(event `LookTowardsHit`
  (params (DirectionOfHit :type "Vector Structure"))
  (`BlackboardComponent.SetValueAsVector` (`AIBlueprintHelperLibrary.GetBlackboard` null) "LastSeenLocation" DirectionOfHit)
  (`KismetSystemLibrary.DrawDebugSphere` DirectionOfHit 20.0 12 (struct :`R` 1.0 :`B` 0.240001 :`A` 1.0) 5.0 1.0))

(fn `UserConstructionScript`)