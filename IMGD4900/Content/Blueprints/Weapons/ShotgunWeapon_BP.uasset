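; Shotgun weapon Blueprint that fires a burst of ShotgunProjectile_BP actors on each Fire event.
; A loop spawns each pellet at the muzzle location offset by the aim vector, oriented along the aim rotation.
; Independent random pitch and yaw offsets create the spread cone, which is asymmetric in pitch, while the random location offset has a zero range.
; The construction script only calls its parent.
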(event `self.Fire`
  (for _ (range 11)
    (`|SpawnActorFromClass` "/Game/Blueprints/Weapons/ShotgunProjectile_BP.ShotgunProjectile_BP_C" (`KismetMathLibrary.MakeTransform` (+ (+ (`SceneComponent.K2_GetComponentLocation` (`self.MuzzleLoc`)) (`self.AimVetor`)) (`KismetMathLibrary.RandomFloatInRange` 0.0 0.0)) (`KismetMathLibrary.MakeRotator` 0.0 (+ (.pitch (`self.AimRotation`)) (`KismetMathLibrary.RandomFloatInRange` -15.0 10.0)) (+ (.yaw (`self.AimRotation`)) (`KismetMathLibrary.RandomFloatInRange` -10.0 10.0)))) "Undefined" "OverrideRootScale" null null)))

(fn `UserConstructionScript`
  (`parent.UserConstructionScript`))